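; Drivable physics tracked vehicle (tank) that characters enter and leave with X, swapping possession.
; Throttle and steer axes become per-side torques on the skeletal mesh's wheel bones for skid steering.
; Each driven tick, wheel bone heights deform two track splines that position instanced links and road wheels.
; Measured left and right speeds scroll the links and spin wheels, sprockets and idlers, while averaged speed drives the speed readout and audio.
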(event `self.ReceiveBeginPlay`
  (bind _trackmesh1 (`self.trackMesh1`))
  (bind _numtracks (`self.numTracks`))
  (bind _wheelmesh (`self.wheelMesh`))
  (bind _wheelrot (`self.wheelRot`))
  (`SceneComponent.SetVisibility` (`self.TextRender1`) true false)
  (`PrimitiveComponent.SetSimulatePhysics` (`self.SkeletalMesh`) true)
  ;[1 1 1] Initial track links population
  (`InstancedStaticMeshComponent.ClearInstances` _trackmesh1)
  (for _index (range (* _numtracks 2))
    (bind _returnvalue (<= _index (- _numtracks 1)))
    (bind (_returnvalue_location _returnvalue_rotation _returnvalue_scale) (`KismetMathLibrary.BreakTransform` (`SplineComponent.GetTransformAtTime` (select `bool` _returnvalue :`false` (`self.SplineTrack2`) :`true` (`self.SplineTrack1`)) (* (`KismetMathLibrary.SelectInt` _index (- _index _numtracks) _returnvalue) (/ 1.0 (`KismetMathLibrary.Conv_IntToDouble` _numtracks))) "World" true true)))
    (`InstancedStaticMeshComponent.AddInstanceWorldSpace` _trackmesh1 (`KismetMathLibrary.MakeTransform` _returnvalue_location _returnvalue_rotation _returnvalue_scale)))
  ;[1 1 1] Setting up wheels
  (`InstancedStaticMeshComponent.ClearInstances` _wheelmesh)
  (for (_array_element _array_index) (`self.driveWheels`)
    (`KismetArrayLibrary.Array_Set` _wheelrot _array_index (`KismetMathLibrary.RandomFloatInRange` 0.0 360.0))
    (bind (_outposition _outrotation) (`SkinnedMeshComponent.TransformFromBoneSpace` :`self` (`self.SkeletalMesh`) :`BoneName` _array_element))
    (bind (_x _y _z) (`KismetMathLibrary.GetAxes` _outrotation))
    (`InstancedStaticMeshComponent.AddInstanceWorldSpace` _wheelmesh (`KismetMathLibrary.MakeTransform` _outposition (`KismetMathLibrary.MakeRotFromXZ` _z (`KismetMathLibrary.RotateAngleAxis` _y (`|GetArrayItem` _wheelrot _array_index) _z))))))

(event `self.ReceiveTick`
  (params (DeltaSeconds :type "Float (single-precision)"))
  (bind _returnvalue (`self.GetControlRotation`))
  (bind _returnvalue_2 (`self.GetInputAxisValue`))
  (bind _tracktime (`self.trackTime`))
  (bind _splinetrack1 (`self.SplineTrack1`))
  (bind _skeletalmesh (`self.SkeletalMesh`))
  (bind _numtracks (`self.numTracks`))
  (bind _saveddriver (`self.savedDriver`))
  (bind _idler1 (`self.idler1`))
  (bind _wheelrot (`self.wheelRot`))
  (bind _skeletalmesh_2 (`self.SkeletalMesh`))
  (bind _sprocket2 (`self.sprocket2`))
  (bind _speedright (`self.speedRight`))
  (bind _speedleft (`self.speedLeft`))
  (bind _idler2 (`self.idler2`))
  (bind _tracktime_2 (`self.trackTime`))
  (bind _tracktime_3 (`self.trackTime`))
  (bind _audio (`self.Audio`))
  (bind _forwardspeed (`self.forwardSpeed`))
  (bind _rootbone (`self.rootBone`))
  (bind _sprocket1 (`self.sprocket1`))
  (bind _overlappingactors (`PrimitiveComponent.GetOverlappingActors` (`self.EntryVolume`) "/Script/Engine.Character"))
  (bind _relativerotation_roll (`KismetMathLibrary.BreakRotator` (`SceneComponent.RelativeRotation` _sprocket2)))
  (bind _relativerotation_roll_2 (`KismetMathLibrary.BreakRotator` (`SceneComponent.RelativeRotation` _idler2)))
  (bind _relativerotation_roll_3 (`KismetMathLibrary.BreakRotator` (`SceneComponent.RelativeRotation` _sprocket1)))
  (bind _relativerotation_roll_4 (`KismetMathLibrary.BreakRotator` (`SceneComponent.RelativeRotation` _idler1)))
  (bind (_relativelocation_x _relativelocation_y _relativelocation_z) (`KismetMathLibrary.BreakVector` (`SceneComponent.RelativeLocation` _splinetrack1)))
  (bind _returnvalue_3 (- (* _numtracks 2) 1))
  (bind (_x _y _z) (`KismetMathLibrary.GetAxes` (`SceneComponent.K2_GetComponentRotation` (`self.SkeletalMesh`))))
  (bind _returnvalue_4 (+ (`|GetArrayItem` _tracktime_2) (* DeltaSeconds (/ (`self.speedRight`) 1163.0))))
  (bind _returnvalue_5 (+ (`|GetArrayItem` _tracktime 1) (* DeltaSeconds (/ (`self.speedLeft`) 1163.0))))
  (if (`self.bDriven`)
    (bind _asplayer_controller (cast `PlayerController` (`self.GetController`)))
    (if (`PlayerController.WasInputKeyJustPressed` _asplayer_controller "X")
      ;[1 1 1] Leaving a vehicle
      (`KismetSystemLibrary.PrintString` "Hello")
      (`self.K2_TeleportTo` :`self` _saveddriver :`DestLocation` (+ (`SceneComponent.K2_GetComponentLocation` (`self.SkeletalMesh`)) (0.0 0.0 250.0)))
      (`Controller.UnPossess` _asplayer_controller)
      (`Controller.Possess` _asplayer_controller _saveddriver)
      (set `self.bDriven` false))
    (`SceneComponent.K2_SetWorldLocationAndRotation` (`self.Camera`) (+ (`SceneComponent.K2_GetComponentLocation` (`self.SkeletalMesh`)) (0.0 0.0 150.0) (* (`KismetMathLibrary.GetForwardVector` _returnvalue) -600.0)) _returnvalue false false)
    (set `self.throttleVal` (`KismetMathLibrary.FInterpTo_Constant` (`self.throttleVal`) (`KismetMathLibrary.SelectFloat` 0.0 (`KismetMathLibrary.SelectFloat` -4.0 -4.0 (> _returnvalue_2 0.0)) (== _returnvalue_2 0.0)) DeltaSeconds 5.0))
    ;[1 1 1] Speed value
    (bind _output_get (set `self.forwardSpeed` (/ (+ (`self.speedLeft`) (`self.speedRight`)) 2.0)))
    (`TextRenderComponent.K2_SetText` (`self.TextRender`) (`KismetTextLibrary.Conv_DoubleToText` (* _output_get 0.036) "HalfToEven"))
    (`KismetArrayLibrary.Array_Set` _tracktime_2 0 (`KismetMathLibrary.SelectFloat` (- _returnvalue_4 1.0) (`KismetMathLibrary.SelectFloat` (+ _returnvalue_4 1.0) _returnvalue_4 (< _returnvalue_4 0.0)) (> _returnvalue_4 1.0)))
    (`KismetArrayLibrary.Array_Set` _tracktime 1 (`KismetMathLibrary.SelectFloat` (- _returnvalue_5 1.0) (`KismetMathLibrary.SelectFloat` (+ _returnvalue_5 1.0) _returnvalue_5 (< _returnvalue_5 0.0)) (> _returnvalue_5 1.0)))
    ;[1 1 1] Spline points Update
    (for (_array_element _array_index) (`self.driveWheels`)
      (bind _outposition (`SkinnedMeshComponent.TransformFromBoneSpace` :`self` _skeletalmesh :`BoneName` _array_element))
      (bind _output_x (`KismetMathLibrary.BreakVector` (`|GetArrayItem` (`self.trackPoints`) _array_index)))
      (bind (_returnvalue_x _returnvalue_y _returnvalue_z) (`KismetMathLibrary.BreakVector` (`KismetMathLibrary.InverseTransformLocation` (`SceneComponent.K2_GetComponentToWorld` _skeletalmesh) _outposition)))
      (bind _returnvalue_6 (- _array_index 1))
      (`SplineComponent.SetLocationAtSplinePoint` (select `bool` (>= (`KismetArrayLibrary.Array_Find` (`self.wheelRight`) _array_element) 0) :`false` (`self.SplineTrack2`) :`true` _splinetrack1) (`KismetMathLibrary.FTrunc` (`|GetArrayItem` (`self.wheelSplinePoints`) _array_index)) (`KismetMathLibrary.MakeVector` _output_x 0.0 (- _returnvalue_z (+ (`self.physWheelRadius`) _relativelocation_z))) "Local" (or (== _returnvalue_6 (`KismetArrayLibrary.Array_Length` (`self.wheelRight`))) (== _returnvalue_6 (`KismetArrayLibrary.Array_Length` (`self.driveWheels`))))))
    ;[1 1 1] tracks deformation
    (for _index (range (+ _returnvalue_3 1))
      (bind _returnvalue_7 (< _index _numtracks))
      (bind _returnvalue_8 (select `bool` _returnvalue_7 :`false` (`self.SplineTrack2`) :`true` (`self.SplineTrack1`)))
      (bind _returnvalue_9 (+ (* (`KismetMathLibrary.SelectInt` _index (- _index _numtracks) _returnvalue_7) (/ 1.0 (`KismetMathLibrary.Conv_IntToDouble` _numtracks))) (`KismetMathLibrary.SelectFloat` (`|GetArrayItem` _tracktime_3) (`|GetArrayItem` _tracktime_3 1) _returnvalue_7)))
      (`InstancedStaticMeshComponent.UpdateInstanceTransform` (`self.trackMesh1`) _index (`KismetMathLibrary.MakeTransform` (.location (`SplineComponent.GetTransformAtTime` _returnvalue_8 (`KismetMathLibrary.SelectFloat` (- _returnvalue_9 1.0) (`KismetMathLibrary.SelectFloat` (+ _returnvalue_9 1.0) _returnvalue_9 (< _returnvalue_9 0.0)) (> _returnvalue_9 1.0)) "World" true false)) (`KismetMathLibrary.MakeRotFromXY` (`KismetMathLibrary.GetForwardVector` (.rotation (`SplineComponent.GetTransformAtTime` _returnvalue_8 (`KismetMathLibrary.SelectFloat` (- _returnvalue_9 1.0) (`KismetMathLibrary.SelectFloat` (+ _returnvalue_9 1.0) _returnvalue_9 (< _returnvalue_9 0.0)) (> _returnvalue_9 1.0)) "World" true false))) (* (`SceneComponent.GetRightVector` _returnvalue_8) -1.0))) true (== _index _returnvalue_3) false))
    ;[1 1 1] Sprocket + Idler
    (`SceneComponent.K2_SetRelativeRotation` _sprocket1 (`KismetMathLibrary.MakeRotator` (mod (+ _relativerotation_roll_3 (* (/ _speedright 169.639999) DeltaSeconds -360.0)) 360.0) 0.0 90.0) false false)
    (`SceneComponent.K2_SetRelativeRotation` _idler1 (`KismetMathLibrary.MakeRotator` (mod (+ _relativerotation_roll_4 (* (/ _speedright 150.789993) DeltaSeconds -360.0)) 360.0) 0.0 90.0) false false)
    (`SceneComponent.K2_SetRelativeRotation` _sprocket2 (`KismetMathLibrary.MakeRotator` (mod (+ _relativerotation_roll (* (/ _speedleft 169.639999) DeltaSeconds 360.0)) 360.0) 0.0 -90.0) false false)
    (`SceneComponent.K2_SetRelativeRotation` _idler2 (`KismetMathLibrary.MakeRotator` (mod (+ _relativerotation_roll_2 (* (/ _speedleft 150.789993) DeltaSeconds 360.0)) 360.0) 0.0 -90.0) false false)
    ;[1 1 1] Road wheels rotation
    (for _index_2 (range (`KismetArrayLibrary.Array_Length` (`self.driveWheels`)))
      (bind _returnvalue_10 (< _index_2 (`KismetArrayLibrary.Array_Length` (`self.wheelRight`))))
      (bind _returnvalue_11 (mod (+ (`|GetArrayItem` _wheelrot _index_2) (* (/ (`KismetMathLibrary.SelectFloat` (`self.speedRight`) (`self.speedLeft`) _returnvalue_10) 197.919998) DeltaSeconds 360.0)) 360.0))
      (`KismetArrayLibrary.Array_Set` _wheelrot _index_2 _returnvalue_11)
      (`InstancedStaticMeshComponent.UpdateInstanceTransform` (`self.wheelMesh`) _index_2 (`KismetMathLibrary.MakeTransform` (+ (`SplineComponent.GetLocationAtSplineInputKey` (select `bool` _returnvalue_10 :`false` (`self.SplineTrack2`) :`true` (`self.SplineTrack1`)) (`|GetArrayItem` (`self.wheelSplinePoints`) _index_2) "World") (* _z 31.5)) (`KismetMathLibrary.MakeRotFromXZ` (`KismetMathLibrary.SelectVector` _y (* _y -1.0) _returnvalue_10) (`KismetMathLibrary.RotateAngleAxis` _z _returnvalue_11 _y))) true true false))
    ;[1 1 1] Getting right- & left-side speeds (for proper tracks motion)
    (bind (_outposition_2 _outrotation) (`SkinnedMeshComponent.TransformFromBoneSpace` :`self` _skeletalmesh_2 :`BoneName` _rootbone :`InPosition` (0.0 0.0 1.2)))
    (bind _returnvalue_12 (`PrimitiveComponent.GetPhysicsLinearVelocityAtPoint` _skeletalmesh_2 _outposition_2 _rootbone))
    (set `self.speedRight` (`KismetMathLibrary.Dot_VectorVector` _returnvalue_12 (`KismetMathLibrary.GetForwardVector` _outrotation)))
    (bind (_outposition_3 _outrotation_2) (`SkinnedMeshComponent.TransformFromBoneSpace` :`self` _skeletalmesh_2 :`BoneName` _rootbone :`InPosition` (0.0 0.0 -1.2)))
    (bind _returnvalue_13 (`PrimitiveComponent.GetPhysicsLinearVelocityAtPoint` _skeletalmesh_2 _outposition_3 _rootbone))
    (set `self.speedLeft` (`KismetMathLibrary.Dot_VectorVector` _returnvalue_13 (`KismetMathLibrary.GetForwardVector` _outrotation_2)))
    ;[1 1 1] Dynamic sound params
    (`AudioComponent.SetFloatParameter` _audio "trackPitch" (`KismetMathLibrary.MapRangeClamped` _forwardspeed 500.0 2000.0 0.7 1.2))
    (`AudioComponent.SetFloatParameter` _audio "trackVol" (`KismetMathLibrary.MapRangeClamped` _forwardspeed 50.0 1000.0 0.0 1.0))
    (`AudioComponent.SetFloatParameter` _audio "enginePitch" (`KismetMathLibrary.MapRangeClamped` _forwardspeed 0.0 2500.0 0.5 1.1))
    (`AudioComponent.SetFloatParameter` _audio "engineVol" (`KismetMathLibrary.MapRangeClamped` (`KismetMathLibrary.Abs` (`self.throttleVal`)) 0.0 4.0 1.0 1.0))
    (else
      ;[1 1 1] Checking for driver when not driven
      (if (> (`KismetArrayLibrary.Array_Length` _overlappingactors) 0)
        (bind _asplayer_controller_2 (cast `PlayerController` (`self.GetInstigatorController` (`|GetArrayItem` _overlappingactors))))
        (if (`PlayerController.WasInputKeyJustPressed` _asplayer_controller_2 "X")
          (set `self.savedDriver` (`Controller.K2_GetPawn` _asplayer_controller_2))
          (`Controller.UnPossess` _asplayer_controller_2)
          (`Controller.Possess` _asplayer_controller_2 self)
          (set `self.bDriven` true)
          (`ActorComponent.SetActive` (`self.Audio`) true true)
          (`KismetSystemLibrary.PrintString` "Driven!"))))))

(event `InputAxis|AxisThrottle`
  (params (AxisValue :type "Float (single-precision)"))
  (bind _returnvalue (`self.GetInputAxisValue`))
  (bind _driveright (`self.driveRight`))
  (bind _driveleft (`self.driveLeft`))
  (bind _skeletalmesh (`self.SkeletalMesh`))
  (bind _returnvalue_2 (`SceneComponent.GetRightVector` _skeletalmesh))
  (bind _returnvalue_3 (* (`self.GetInputAxisValue`) (`self.throttleVal`)))
  ;[1 1 1] Forces for actual movement
  (set `self.driveLeft` (`KismetMathLibrary.SelectFloat` _returnvalue_3 (`KismetMathLibrary.SelectFloat` 0.0 -4.0 (> _returnvalue 0.0)) (== _returnvalue 0.0)))
  (set `self.driveRight` (`KismetMathLibrary.SelectFloat` _returnvalue_3 (`KismetMathLibrary.SelectFloat` 0.0 -4.0 (< _returnvalue 0.0)) (== _returnvalue 0.0)))
  (for _array_element (`self.driveWheels`)
    (bind _returnvalue_4 (`PrimitiveComponent.GetPhysicsAngularVelocityInDegrees` _skeletalmesh _array_element))
    (bind _returnvalue_5 (`KismetMathLibrary.SelectFloat` _driveright _driveleft (>= (`KismetArrayLibrary.Array_Find` (`self.wheelRight`) _array_element) 0)))
    (`PrimitiveComponent.AddTorqueInDegrees` _skeletalmesh (`KismetMathLibrary.SelectVector` (* _returnvalue_4 (`KismetMathLibrary.SelectFloat` -400000.0 0.0 (> (`KismetMathLibrary.Dot_VectorVector` _returnvalue_4 _returnvalue_2) 0.0))) (* _returnvalue_2 (* _returnvalue_5 -360.0 200000.0)) (or (and (== _returnvalue_5 0.0) (or (!= _driveright 0.0) (!= _driveleft 0.0))) (and (> (`self.forwardSpeed`) 10.0) (< (`self.GetInputAxisValue`) 0.0)))) _array_element false)))

(event `self.ReceiveDestroyed`
  (`KismetSystemLibrary.PrintString` "Tank removed!"))

(fn `UserConstructionScript`)